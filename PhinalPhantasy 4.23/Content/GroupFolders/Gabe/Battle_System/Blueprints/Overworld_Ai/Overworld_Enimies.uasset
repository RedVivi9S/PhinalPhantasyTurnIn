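; Overworld enemy that chases the player through AI perception and starts a battle level when the player overlaps it.
; Perception updates feed target and line-of-sight state to AIC_Overworld, with a delayed timer clearing the target after sight is lost.
; On contact it saves potions, chests, player state and the spawner's other enemies, omitting itself.
; It then passes its battle data and camera index to the game instance before loading the level.
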(event `self.ReceiveActorBeginOverlap`
  (params (OtherActor :type "Actor Object Reference"))
  (cast `/Game/ThirdPersonBP/Blueprints/ThirdPersonCharacter` OtherActor)
  (`self.Save_Game`)
  (`self.SetAiParty`)
  (`GameplayStatics.OpenLevel` (`self.LevelName`)))

(event `Set Transform`
  (params (Location :type "Vector Structure") (Rotation :type "Rotator Structure") (Scale :type "Vector Structure"))
  (`self.K2_SetActorRelativeLocation` Location false true)
  (`self.K2_SetActorRotation` Rotation)
  (`self.SetActorScale3D` Scale))

(event `self.Sense.OnTargetPerceptionUpdated`
  (params (Actor :type "Actor Object Reference") (Stimulus :type "AIStimulus Structure"))
  (bind _asaic_overworld (cast `/Game/GroupFolders/Gabe/Battle_System/Blueprints/Overworld_Ai/AIC_Overworld` (`self.GetController`) :!pure true))
  (bind _asthird_person_character (cast `/Game/ThirdPersonBP/Blueprints/ThirdPersonCharacter` Actor))
  (set `self.Target` _asthird_person_character)
  (if (`.bSuccessfullySensed` (break `AIStimulus` Stimulus))
    (`KismetSystemLibrary.K2_ClearAndInvalidateTimerHandle` (`self.Target Lost Timer`))
    (`/Game/GroupFolders/Gabe/Battle_System/Blueprints/Overworld_Ai/AIC_Overworld.Update_Target_Actor` _asaic_overworld (`self.Target`))
    (`/Game/GroupFolders/Gabe/Battle_System/Blueprints/Overworld_Ai/AIC_Overworld.Update_Has_Line_Of_Sight` _asaic_overworld true)
    (else
      (bind _returnvalue (`KismetSystemLibrary.K2_SetTimerDelegate` (delegate `Lost Target`) 5.0))
      (set `self.Target Lost Timer` _returnvalue)
      (`/Game/GroupFolders/Gabe/Battle_System/Blueprints/Overworld_Ai/AIC_Overworld.Update_Has_Line_Of_Sight` (cast `/Game/GroupFolders/Gabe/Battle_System/Blueprints/Overworld_Ai/AIC_Overworld` (`self.GetController`) :!pure true) false))))

(event `Lost Target`
  (set `self.Target` null)
  (`/Game/GroupFolders/Gabe/Battle_System/Blueprints/Overworld_Ai/AIC_Overworld.Update_Target_Actor` (cast `/Game/GroupFolders/Gabe/Battle_System/Blueprints/Overworld_Ai/AIC_Overworld` (`self.GetController`) :!pure true) null))

(fn `Save_Game`
  (bind _returnvalue (`GameplayStatics.GetPlayerCharacter` 0))
  (bind _spawner (`self.Spawner`))
  (bind _returnvalue_2 (`GameplayStatics.CreateSaveGameObject` "/Game/GroupFolders/Gabe/Battle_System/SaveGame_01.SaveGame_01_C"))
  (bind _output_get (set `self.Save Game Sub` _returnvalue_2))
  (bind _outactors (`GameplayStatics.GetAllActorsOfClass` "/Game/GroupFolders/Ged/Items/Potion_Spawner.Potion_Spawner_C"))
  (for (_array_element _array_index) _outactors
    (bind _aspotion_spawner (cast `/Game/GroupFolders/Ged/Items/Potion_Spawner` _array_element))
    (`KismetArrayLibrary.Array_Set` (`/Game/GroupFolders/Gabe/Battle_System/SaveGame_01.PotionNums` _output_get) _array_index (`/Game/GroupFolders/Ged/Items/Potion_Spawner.NumPotions` _aspotion_spawner) true))
  (bind _outactors_2 (`GameplayStatics.GetAllActorsOfClass` "/Game/GroupFolders/Ged/Containers/Chest.Chest_C"))
  (for (_array_element_2 _array_index_2) _outactors_2
    (`KismetArrayLibrary.Array_Set` (`/Game/GroupFolders/Gabe/Battle_System/SaveGame_01.Chests` _output_get) _array_index_2 _array_element_2 true)
    (`KismetArrayLibrary.Array_Set` (`/Game/GroupFolders/Gabe/Battle_System/SaveGame_01.Inventories` _output_get) _array_index_2 (make `/Game/GroupFolders/Ged/Inventories` (`/Game/GroupFolders/Ged/InventoryComponet.Inventory` (`/Game/GroupFolders/Ged/Containers/Container_Parent.InventoryComponet` _array_element_2))) true))
  (set `/Game/GroupFolders/Gabe/Battle_System/SaveGame_01.Controller Rotation` (`self.K2_GetActorRotation` (`GameplayStatics.GetPlayerController` 0)) _output_get)
  (set `/Game/GroupFolders/Gabe/Battle_System/SaveGame_01.Spawners` _spawner _output_get)
  (set `/Game/GroupFolders/Gabe/Battle_System/SaveGame_01.PlayerTransform` (`KismetMathLibrary.MakeTransform` (`self.K2_GetActorLocation` _returnvalue) (`self.K2_GetActorRotation` _returnvalue) (`self.GetActorScale3D` _returnvalue)) _output_get)
  (`/Game/ThirdPersonBP/Blueprints/ThirdPersonCharacter.Save Inventory` (cast `/Game/ThirdPersonBP/Blueprints/ThirdPersonCharacter` _returnvalue :!pure true))
  (for _array_element_3 (`/Game/GroupFolders/Gabe/Battle_System/AiSpawner/AiSpawner.SpawnersChildren` _spawner)
    (`/Engine/EditorBlueprintResources/StandardMacros.IsValid` _array_element_3
      (:`Is Valid`
        (if (!= self _array_element_3)
          (`KismetArrayLibrary.Array_Add` (`/Game/GroupFolders/Gabe/Battle_System/SaveGame_01.Ai Locations` _output_get) (`KismetMathLibrary.MakeTransform` (`self.K2_GetActorLocation` _array_element_3) (`self.K2_GetActorRotation` _array_element_3) (`self.GetActorScale3D` _array_element_3)))))))
  (`GameplayStatics.SaveGameToSlot` (`self.Save Game Sub`) (`/Game/GroupFolders/Gabe/Battle_System/RPG_GameInstance.GameSaveName` (cast `/Game/GroupFolders/Gabe/Battle_System/RPG_GameInstance` (`GameplayStatics.GetGameInstance`) :!pure true))))

(fn `SetAiParty`
  (bind _mesh (`self.Mesh`))
  (bind _asrpg_game_instance (cast `/Game/GroupFolders/Gabe/Battle_System/RPG_GameInstance` (`GameplayStatics.GetGameInstance`) :!pure true))
  (set `/Game/GroupFolders/Gabe/Battle_System/RPG_GameInstance.Ai_Party` (make `/Game/GroupFolders/Gabe/Battle_System/Ai_Data` (`self.EnemyHp`) (`self.Exp`) (`self.EnemyStats`) (`KismetMathLibrary.RandomIntegerInRange` 0 2) (`SkinnedMeshComponent.SkeletalMesh` _mesh) (`GameplayStatics.GetObjectClass` (`SkeletalMeshComponent.GetAnimInstance` _mesh))) _asrpg_game_instance)
  (set `/Game/GroupFolders/Gabe/Battle_System/RPG_GameInstance.CameraNum` (`self.LocationIndex`) _asrpg_game_instance))

(fn `UserConstructionScript`)