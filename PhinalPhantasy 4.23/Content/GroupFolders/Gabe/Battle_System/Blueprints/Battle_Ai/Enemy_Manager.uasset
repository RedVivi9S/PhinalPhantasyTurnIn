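; Enemy party manager for turn-based RPG battles, active only if its camera index matches the game instance's CameraNum.
; Spawns enemies from the instance's AiParty data, rotates their turns and relays targets to them.
; Handles the player's party-wide super move, with doubled damage against a lone survivor.
; Tracks deaths, reports experience and turn changes through a Mediator, and opens WinScreen when all enemies are dead.
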(event `UpdateParty`
  (for (_array_element _array_index) (`self.Enemies`)
    (`/Engine/EditorBlueprintResources/StandardMacros.IsValid` _array_element
      (:`Is Not Valid`
        (`KismetArrayLibrary.Array_Set` (`self.Are Dead?`) _array_index true)))))

(event `self.ReceiveBeginPlay`
  (bind _asrpg_game_instance (cast `/Game/GroupFolders/Gabe/Battle_System/RPG_GameInstance` (`GameplayStatics.GetGameInstance`) :!pure true))
  (bind (_ai_party_hp _ai_party_exp _ai_party_stats _ai_party_numai _ai_party_skelebones _ai_party_animations) (break `/Game/GroupFolders/Gabe/Battle_System/Ai_Data` (`/Game/GroupFolders/Gabe/Battle_System/RPG_GameInstance.Ai_Party` (cast `/Game/GroupFolders/Gabe/Battle_System/RPG_GameInstance` (`GameplayStatics.GetGameInstance`) :!pure true))))
  (bind (_ai_party_hp_2 _ai_party_exp_2 _ai_party_stats_2 _ai_party_numai_2) (break `/Game/GroupFolders/Gabe/Battle_System/Ai_Data` (`/Game/GroupFolders/Gabe/Battle_System/RPG_GameInstance.Ai_Party` _asrpg_game_instance)))
  (if (== (`/Game/GroupFolders/Gabe/Battle_System/RPG_GameInstance.CameraNum` _asrpg_game_instance) (`self.CameraIndex`))
    (for _index (range (+ _ai_party_numai_2 1))
      (bind _returnvalue (`AIBlueprintHelperLibrary.SpawnAIFromClass` "/Game/GroupFolders/Gabe/Battle_System/Blueprints/Battle_Ai/Ai_1-0/Enemy.Enemy_C" "/Game/GroupFolders/Gabe/Battle_System/Blueprints/Battle_Ai/Ai_1-0/BTT_Ai_1-0.BTT_Ai_1-0" (`|GetArrayItem` (`self.Location`) _index) (`|GetArrayItem` (`self.Rotations`) _index)))
      (bind _asenemy (cast `/Game/GroupFolders/Gabe/Battle_System/Blueprints/Battle_Ai/Ai_1-0/Enemy` _returnvalue))
      (set `/Game/GroupFolders/Gabe/Battle_System/Blueprints/Battle_Ai/Ai_1-0/Enemy.Manager` self _asenemy)
      (bind _output_get (set `/Game/GroupFolders/Gabe/Battle_System/Blueprints/Battle_Ai/Ai_1-0/Enemy.Index` _index _asenemy))
      (set `/Game/GroupFolders/Gabe/Battle_System/Blueprints/Battle_Ai/Ai_1-0/Enemy.Hp` _ai_party_hp _asenemy)
      (set `/Game/GroupFolders/Gabe/Battle_System/Blueprints/Battle_Ai/Ai_1-0/Enemy.Stats` _ai_party_stats _asenemy)
      (set `/Game/GroupFolders/Gabe/Battle_System/Blueprints/Battle_Ai/Ai_1-0/Enemy.Exp` _ai_party_exp _asenemy)
      (`/Game/GroupFolders/Gabe/Battle_System/Blueprints/Battle_Ai/Ai_1-0/AIC_Ai_1-0.Update_Mediator` (cast `/Game/GroupFolders/Gabe/Battle_System/Blueprints/Battle_Ai/Ai_1-0/AIC_Ai_1-0` (`Pawn.GetController` _asenemy) :!pure true) (`self.Mediator`))
      (`KismetArrayLibrary.Array_Insert` (`self.Enemies`) _asenemy _output_get)
      (`KismetArrayLibrary.Array_Add` (`self.Are Dead?`))
      (bind _mesh (`Character.Mesh` _asenemy))
      (`SkinnedMeshComponent.SetSkinnedAssetAndUpdate` _mesh _ai_party_skelebones true)
      (`SkeletalMeshComponent.SetAnimInstanceClass` _mesh _ai_party_animations))
    (bind _output_get_2 (set `self.Attacker` (`|GetArrayItem` (`self.Enemies`))))
    (bind (_stats_attack _stats_defense _stats_speed) (break `/Game/GroupFolders/Gabe/Battle_System/Stats` (`/Game/GroupFolders/Gabe/Battle_System/Blueprints/Battle_Ai/Ai_1-0/Enemy.Stats` _output_get_2)))
    (set `self.Speed` _stats_speed)
    (else
      (`self.K2_DestroyActor`))))

(event `Ai Turn`
  (bind _attacker (`self.Attacker`))
  (`self.Update Enemy`)
  (`/Engine/EditorBlueprintResources/StandardMacros.IsValid` _attacker
    (:`Is Valid`
      (`/Game/GroupFolders/Gabe/Battle_System/Blueprints/Battle_Ai/Ai_1-0/Enemy.Update My Turn` _attacker)
      (bind _asmediator (cast `/Game/GroupFolders/Gabe/Battle_System/Blueprints/Battle_Ai/Mediator` (`self.Mediator`)))
      (`/Game/GroupFolders/Gabe/Battle_System/Blueprints/Battle_Ai/Mediator.Ai To Player` _asmediator))
    (:`Is Not Valid`
      (`self.UpdateParty`)
      (`self.CheckParty`)
      (`KismetSystemLibrary.Delay` 1.0)
      (`self.Ai Turn`))))

(event `Update Targets`
  (params (Target :type "Actor Object Reference"))
  (for _array_element (`self.Enemies`)
    (`/Engine/EditorBlueprintResources/StandardMacros.IsValid` _array_element
      (:`Is Valid`
        (`/Game/GroupFolders/Gabe/Battle_System/Blueprints/Battle_Ai/Ai_1-0/Enemy.Update Target` _array_element Target)))))

(event `Update Still Alive`
  (params (Index :type Integer) (Exp :type "Float (double-precision)"))
  (`KismetSystemLibrary.Delay` 0.5)
  (`GameplayStatics.PlaySound2D` "/Game/GroupFolders/Mason/SFX/EnemyDeath.EnemyDeath" 1.0 1.0 0.0 null null)
  (`/Game/GroupFolders/Gabe/Battle_System/Blueprints/Battle_Ai/Mediator.Update Exp` (cast `/Game/GroupFolders/Gabe/Battle_System/Blueprints/Battle_Ai/Mediator` (`self.Mediator`) :!pure true) Exp)
  (`KismetArrayLibrary.Array_Set` (`self.Are Dead?`) Index true)
  (`self.CheckParty`))

(event `CheckParty`
  (for _array_element (`self.Are Dead?`)
    (set `self.Loss` (and _array_element (`self.Loss`))))
  (if (`self.Loss`)
    (if (`self.Battle Over`)
      (set `self.Battle Over` false)
      (`/Game/GroupFolders/Gabe/Battle_System/Blueprints/Battle_Ai/Mediator.End_Battle` (cast `/Game/GroupFolders/Gabe/Battle_System/Blueprints/Battle_Ai/Mediator` (`self.Mediator`) :!pure true))
      (`KismetSystemLibrary.Delay` 0.2)
      (`GameplayStatics.OpenLevel` "WinScreen"))
    (else
      (set `self.Loss` true))))

(event `SuperMove`
  (params (`Player Stats` :type "/Game/GroupFolders/Gabe/Battle_System/Stats Structure") (`Player Weapon` :type "/Game/GroupFolders/Gabe/Battle_System/Weapon Structure"))
  (set `self.Player Stats` `Player Stats`)
  (set `self.Player Weapon` `Player Weapon`)
  (for _array_element (`self.Are Dead?`)
    (if (not _array_element)
      (`/Engine/EditorBlueprintResources/StandardMacros.IncrementInt` (`self.Total Alive`))))
  (if (> (`self.Total Alive`) 2)
    (for _array_element_2 (`self.Enemies`)
      (`self.Damage Calc` _array_element_2)
      (`GameplayStatics.ApplyDamage` _array_element_2 (`self.Damage`)))
    (`KismetSystemLibrary.Delay` 1.0)
    (`self.Update Battle Msg`)
    (`KismetSystemLibrary.Delay` 5.0)
    (`Widget.RemoveFromParent` (`self.Battle Msg`))
    (set `self.Damage` 0.0)
    (`self.CheckParty`)
    (`/Game/GroupFolders/Gabe/Battle_System/Blueprints/Battle_Ai/Mediator.Update PlayerTurn` (cast `/Game/GroupFolders/Gabe/Battle_System/Blueprints/Battle_Ai/Mediator` (`self.Mediator`) :!pure true))
    (elif (> (`self.Total Alive`) 1)
      (for _array_element_3 (`self.Enemies`)
        (`/Engine/EditorBlueprintResources/StandardMacros.IsValid` _array_element_3
          (:`Is Valid`
            (`self.Damage Calc` _array_element_3)
            (bind _output_get (set `self.Damage` (* (`self.Damage`) 1.0)))
            (`GameplayStatics.ApplyDamage` _array_element_3 _output_get))))
      (`KismetSystemLibrary.Delay` 1.0)
      (`self.Update Battle Msg`)
      (`KismetSystemLibrary.Delay` 5.0)
      (set `self.Damage` 0.0)
      (`Widget.RemoveFromParent` (`self.Battle Msg`))
      (`self.CheckParty`)
      (`/Game/GroupFolders/Gabe/Battle_System/Blueprints/Battle_Ai/Mediator.Update PlayerTurn` (cast `/Game/GroupFolders/Gabe/Battle_System/Blueprints/Battle_Ai/Mediator` (`self.Mediator`) :!pure true))
      (else
        (for _array_element_4 (`self.Enemies`)
          (`/Engine/EditorBlueprintResources/StandardMacros.IsValid` _array_element_4
            (:`Is Valid`
              (`self.Damage Calc` _array_element_4)
              (bind _output_get_2 (set `self.Damage` (* (`self.Damage`) 2.0)))
              (`GameplayStatics.ApplyDamage` _array_element_4 _output_get_2))))
        (`KismetSystemLibrary.Delay` 1.0)
        (`self.Update Battle Msg`)
        (`KismetSystemLibrary.Delay` 5.0)
        (set `self.Damage` 0.0)
        (`Widget.RemoveFromParent` (`self.Battle Msg`))
        (`self.CheckParty`)
        (`/Game/GroupFolders/Gabe/Battle_System/Blueprints/Battle_Ai/Mediator.Update PlayerTurn` (cast `/Game/GroupFolders/Gabe/Battle_System/Blueprints/Battle_Ai/Mediator` (`self.Mediator`) :!pure true))))))

(fn `Damage Calc`
  (params (Enemy :type "/Game/GroupFolders/Gabe/Battle_System/Blueprints/Battle_Ai/Ai_1-0/Enemy Object Reference"))
  (bind _player_stats_attack (break `/Game/GroupFolders/Gabe/Battle_System/Stats` (`self.Player Stats`)))
  (bind (_stats_attack _stats_defense) (break `/Game/GroupFolders/Gabe/Battle_System/Stats` (`/Game/GroupFolders/Gabe/Battle_System/Blueprints/Battle_Ai/Ai_1-0/Enemy.Stats` Enemy)))
  (bind (_player_weapon_name _player_weapon_damage _player_weapon_mod) (break `/Game/GroupFolders/Gabe/Battle_System/Weapon` (`self.Player Weapon`)))
  (bind (_player_weapon_name_2 _player_weapon_damage_2 _player_weapon_mod_2) (break `/Game/GroupFolders/Gabe/Battle_System/Weapon` (`self.Player Weapon`)))
  (bind _returnvalue (- _player_stats_attack _stats_defense))
  (if (> _returnvalue 0)
    (set `self.Damage` (`KismetMathLibrary.Conv_IntToDouble` (+ _player_weapon_mod_2 (* _player_weapon_damage _returnvalue))))
    (else
      (set `self.Damage` (`KismetMathLibrary.Conv_IntToDouble` (- (+ _player_weapon_damage _player_weapon_mod) (/ _stats_defense 2)))))))

(fn `Update Battle Msg`
  (bind _returnvalue (`|CreateWidget` "/Game/GroupFolders/Gabe/Battle_System/Widgets/BattleMsg.BattleMsg_C"))
  (bind _output_get (set `self.Battle Msg` _returnvalue))
  (set `/Game/GroupFolders/Gabe/Battle_System/Widgets/BattleMsg.Attacker` "Player" _output_get)
  (set `/Game/GroupFolders/Gabe/Battle_System/Widgets/BattleMsg.Reciver` "Enemy Party" _output_get)
  (set `/Game/GroupFolders/Gabe/Battle_System/Widgets/BattleMsg.Damage` (`self.Damage`) _output_get)
  (`/Game/GroupFolders/Gabe/Battle_System/Widgets/BattleMsg.Update` _output_get)
  (`UserWidget.AddToViewport` _output_get 0))

(fn `Update Enemy`
  (bind _enemies (`self.Enemies`))
  (`/Engine/EditorBlueprintResources/StandardMacros.IncrementInt` (`self.Index`)
    (:`  `
      (if (< (`self.Index`) (`KismetArrayLibrary.Array_Length` (`self.Enemies`)))
        (set `self.Attacker` (`|GetArrayItem` _enemies (`self.Index`)))
        (else
          (bind _output_get (set `self.Index` 0))
          (set `self.Attacker` (`|GetArrayItem` _enemies _output_get)))))))

(fn `UserConstructionScript`)