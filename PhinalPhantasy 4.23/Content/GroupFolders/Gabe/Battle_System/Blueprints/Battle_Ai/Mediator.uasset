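; Battle mediator actor that coordinates turns between the player manager and an enemy or boss manager in RPG combat.
; If its camera index matches the game instance's, it opens the battle UI, registers with the battle controller and gives first turn by Speed, otherwise destroying itself.
; Turn handoffs use end-turn flags, re-checked every two seconds until set.
; It also relays player attacks, experience gains and battle end.
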(event `self.ReceiveBeginPlay`
  (bind _enemy_manger (`self.Enemy_Manger`))
  (bind _player (`/Game/GroupFolders/Gabe/Battle_System/Blueprints/Battle_Ai/Player/Player_Manager.Player` (cast `/Game/GroupFolders/Gabe/Battle_System/Blueprints/Battle_Ai/Player/Player_Manager` (`self.BattleManager`) :!pure true)))
  (if (== (`/Game/GroupFolders/Gabe/Battle_System/RPG_GameInstance.CameraNum` (cast `/Game/GroupFolders/Gabe/Battle_System/RPG_GameInstance` (`GameplayStatics.GetGameInstance`) :!pure true)) (`self.CameraIndex`))
    (`GameplayStatics.PlaySound2D` "/Game/GroupFolders/Mason/SFX/EnteringBattle.EnteringBattle" 1.0 1.0 1.0 null null)
    (`KismetSystemLibrary.Delay` 1.3)
    (bind _returnvalue (`|CreateWidget` "/Game/GroupFolders/Mason/UI/BattleStats.BattleStats_C"))
    (bind _output_get (set `self.BattleStats` _returnvalue))
    (`/Game/GroupFolders/Mason/UI/BattleStats.Start Battle` _output_get)
    (`UserWidget.AddToViewport` _output_get 0)
    (bind _asbattle_contorller (cast `/Game/GroupFolders/Gabe/Battle_System/Blueprints/Battle_Ai/Player/Battle_Contorller` (`GameplayStatics.GetPlayerController` 0)))
    (set `/Game/GroupFolders/Gabe/Battle_System/Blueprints/Battle_Ai/Player/Battle_Contorller.Mediator` self _asbattle_contorller)
    (`KismetSystemLibrary.Delay` 0.2)
    (`|ExecutionSequence`
      (:`then_0`
        (bind _asenemy_manager (cast `/Game/GroupFolders/Gabe/Battle_System/Blueprints/Battle_Ai/Enemy_Manager` _enemy_manger))
        (`/Game/GroupFolders/Gabe/Battle_System/Blueprints/Battle_Ai/Enemy_Manager.Update Targets` _asenemy_manager _player)
        (`self.WhoFirst` (`/Game/GroupFolders/Gabe/Battle_System/Blueprints/Battle_Ai/Enemy_Manager.Speed` _asenemy_manager)))
      (:`then_1`
        (bind _asboss_manager (cast `/Game/GroupFolders/Gabe/Battle_System/Blueprints/Battle_Ai/Boss_Manager` _enemy_manger))
        (`/Game/GroupFolders/Gabe/Battle_System/Blueprints/Battle_Ai/Boss_Manager.Update Targets` _asboss_manager _player)
        (`self.WhoFirst` (`/Game/GroupFolders/Gabe/Battle_System/Blueprints/Battle_Ai/Boss_Manager.Speed` _asboss_manager))))
    (else
      (`self.K2_DestroyActor`))))

(event `Player To Ai`
  (bind _enemy_manger (`self.Enemy_Manger`))
  (if (`self.End_PlayerTurn`)
    (if (not (`self.Finished`))
      (`|ExecutionSequence`
        (:`then_0`
          (bind _asenemy_manager (cast `/Game/GroupFolders/Gabe/Battle_System/Blueprints/Battle_Ai/Enemy_Manager` _enemy_manger))
          (`/Game/GroupFolders/Gabe/Battle_System/Blueprints/Battle_Ai/Enemy_Manager.Ai Turn` _asenemy_manager))
        (:`then_1`
          (bind _asboss_manager (cast `/Game/GroupFolders/Gabe/Battle_System/Blueprints/Battle_Ai/Boss_Manager` _enemy_manger))
          (`/Game/GroupFolders/Gabe/Battle_System/Blueprints/Battle_Ai/Boss_Manager.Ai Turn` _asboss_manager)))
      (set `self.Finished` true)
      (set `self.End_PlayerTurn` false))
    (else
      (`KismetSystemLibrary.Delay` 2.0)
      (`self.Player To Ai`))))

(event `Ai To Player`
  (if (`self.End_AiTurn`)
    (if (not (`self.Finished`))
      (bind _asplayer_manager (cast `/Game/GroupFolders/Gabe/Battle_System/Blueprints/Battle_Ai/Player/Player_Manager` (`self.BattleManager`)))
      (`/Game/GroupFolders/Gabe/Battle_System/Blueprints/Battle_Ai/Player/Player_Manager.Run_Turn` _asplayer_manager)
      (set `self.Finished` true)
      (set `self.End_AiTurn` false))
    (else
      (`KismetSystemLibrary.Delay` 2.0)
      (`self.Ai To Player`))))

(event `Update PlayerTurn`
  (set `self.End_PlayerTurn` true)
  (set `self.Finished` false))

(event `Update AiTurn`
  (set `self.End_AiTurn` true)
  (set `self.Finished` false))

(event `Update Exp`
  (params (Exp :type "Float (double-precision)"))
  (bind _asplayer (cast `/Game/GroupFolders/Gabe/Battle_System/Blueprints/Battle_Ai/Player/Player` (`/Game/GroupFolders/Gabe/Battle_System/Blueprints/Battle_Ai/Player/Player_Manager.Player` (cast `/Game/GroupFolders/Gabe/Battle_System/Blueprints/Battle_Ai/Player/Player_Manager` (`self.BattleManager`) :!pure true)) :!pure true))
  (set `/Game/GroupFolders/Gabe/Battle_System/Blueprints/Battle_Ai/Player/Player.ExpGained` (+ (`/Game/GroupFolders/Gabe/Battle_System/Blueprints/Battle_Ai/Player/Player.ExpGained` _asplayer) Exp) _asplayer))

(event `End_Battle`
  (`/Game/GroupFolders/Gabe/Battle_System/Blueprints/Battle_Ai/Player/Player_Manager.End_Battle` (cast `/Game/GroupFolders/Gabe/Battle_System/Blueprints/Battle_Ai/Player/Player_Manager` (`self.BattleManager`) :!pure true)))

(event `PlayerAttack`
  (`/Game/GroupFolders/Gabe/Battle_System/Blueprints/Battle_Ai/Player/Player_Manager.PlayerAttack` (cast `/Game/GroupFolders/Gabe/Battle_System/Blueprints/Battle_Ai/Player/Player_Manager` (`self.BattleManager`) :!pure true)))

(fn `UserConstructionScript`)

(fn `WhoFirst`
  (params (Speed :type Integer))
  (bind _enemy_manger (`self.Enemy_Manger`))
  (bind (_stats_attack _stats_defense _stats_speed) (break `/Game/GroupFolders/Gabe/Battle_System/Stats` (`/Game/GroupFolders/Gabe/Battle_System/RPG_GameInstance.Stats` (cast `/Game/GroupFolders/Gabe/Battle_System/RPG_GameInstance` (`GameplayStatics.GetGameInstance`) :!pure true))))
  (if (>= Speed _stats_speed)
    (`|ExecutionSequence`
      (:`then_0`
        (bind _asenemy_manager (cast `/Game/GroupFolders/Gabe/Battle_System/Blueprints/Battle_Ai/Enemy_Manager` _enemy_manger))
        (`/Game/GroupFolders/Gabe/Battle_System/Blueprints/Battle_Ai/Enemy_Manager.Ai Turn` _asenemy_manager))
      (:`then_1`
        (bind _asboss_manager (cast `/Game/GroupFolders/Gabe/Battle_System/Blueprints/Battle_Ai/Boss_Manager` _enemy_manger))
        (`/Game/GroupFolders/Gabe/Battle_System/Blueprints/Battle_Ai/Boss_Manager.Ai Turn` _asboss_manager)))
    (else
      (`/Game/GroupFolders/Gabe/Battle_System/Blueprints/Battle_Ai/Player/Player_Manager.Run_Turn` (cast `/Game/GroupFolders/Gabe/Battle_System/Blueprints/Battle_Ai/Player/Player_Manager` (`self.BattleManager`) :!pure true)))))