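; Manager for a turn-based boss battle that spawns one boss when the GameInstance camera number matches its index, otherwise destroys itself.
; It configures the boss's stats, mesh and animations from the GameInstance's AI party data.
; It relays turns, targets and experience through the Mediator, opening WinScreen when BattleOver is set.
; SuperMove calculates damage but zeroes it before showing the battle message, never applying it, then returns the turn.
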(event `self.ReceiveBeginPlay`
  (bind (_ai_party_hp _ai_party_exp _ai_party_stats _ai_party_numai _ai_party_skelebones _ai_party_animations) (break `/Game/GroupFolders/Gabe/Battle_System/Ai_Data` (`/Game/GroupFolders/Gabe/Battle_System/RPG_GameInstance.Ai_Party` (cast `/Game/GroupFolders/Gabe/Battle_System/RPG_GameInstance` (`GameplayStatics.GetGameInstance`) :!pure true))))
  (if (== (`/Game/GroupFolders/Gabe/Battle_System/RPG_GameInstance.CameraNum` (cast `/Game/GroupFolders/Gabe/Battle_System/RPG_GameInstance` (`GameplayStatics.GetGameInstance`) :!pure true)) (`self.CameraIndex`))
    (bind _returnvalue (`AIBlueprintHelperLibrary.SpawnAIFromClass` "/Game/GroupFolders/Gabe/Battle_System/Blueprints/Battle_Ai/Ai_1-0/Boss.Boss_C" "/Game/GroupFolders/Gabe/Battle_System/Blueprints/Battle_Ai/Ai_1-0/BTT_Ai_1-Mini.BTT_Ai_1-Mini" (`self.Location`) (`self.Rotation`)))
    (bind _asboss (cast `/Game/GroupFolders/Gabe/Battle_System/Blueprints/Battle_Ai/Ai_1-0/Boss` _returnvalue))
    (`self.SetActorScale3D` _asboss (`self.Scale`))
    (set `/Game/GroupFolders/Gabe/Battle_System/Blueprints/Battle_Ai/Ai_1-0/Boss.Manager` self _asboss)
    (set `/Game/GroupFolders/Gabe/Battle_System/Blueprints/Battle_Ai/Ai_1-0/Boss.Hp` _ai_party_hp _asboss)
    (set `/Game/GroupFolders/Gabe/Battle_System/Blueprints/Battle_Ai/Ai_1-0/Boss.Stats` _ai_party_stats _asboss)
    (set `/Game/GroupFolders/Gabe/Battle_System/Blueprints/Battle_Ai/Ai_1-0/Boss.Exp` _ai_party_exp _asboss)
    (`/Game/GroupFolders/Gabe/Battle_System/Blueprints/Battle_Ai/Ai_1-0/Boss_Controller.Update_Mediator` (cast `/Game/GroupFolders/Gabe/Battle_System/Blueprints/Battle_Ai/Ai_1-0/Boss_Controller` (`Pawn.GetController` _asboss) :!pure true) (`self.Mediator`))
    (bind _output_get (set `self.Enemies` _asboss))
    (set `self.Attacker` _output_get)
    (bind (_stats_attack _stats_defense _stats_speed) (break `/Game/GroupFolders/Gabe/Battle_System/Stats` (`/Game/GroupFolders/Gabe/Battle_System/Blueprints/Battle_Ai/Ai_1-0/Boss.Stats` _output_get)))
    (set `self.Speed` _stats_speed)
    (bind _mesh (`Character.Mesh` _asboss))
    (`SkinnedMeshComponent.SetSkinnedAssetAndUpdate` _mesh _ai_party_skelebones true)
    (`SkeletalMeshComponent.SetAnimInstanceClass` _mesh _ai_party_animations)
    (else
      (`self.K2_DestroyActor`))))

(event `Ai Turn`
  (bind _attacker (`self.Attacker`))
  (`/Engine/EditorBlueprintResources/StandardMacros.IsValid` _attacker
    (:`Is Valid`
      (`/Game/GroupFolders/Gabe/Battle_System/Blueprints/Battle_Ai/Ai_1-0/Boss.Update My Turn` _attacker)
      (bind _asmediator (cast `/Game/GroupFolders/Gabe/Battle_System/Blueprints/Battle_Ai/Mediator` (`self.Mediator`)))
      (`/Game/GroupFolders/Gabe/Battle_System/Blueprints/Battle_Ai/Mediator.Ai To Player` _asmediator))
    (:`Is Not Valid`
      (`self.CheckParty`))))

(event `Update Targets`
  (params (Target :type "Actor Object Reference"))
  (bind _enemies (`self.Enemies`))
  (`/Engine/EditorBlueprintResources/StandardMacros.IsValid` _enemies
    (:`Is Valid`
      (`/Game/GroupFolders/Gabe/Battle_System/Blueprints/Battle_Ai/Ai_1-0/Boss.Update Target` _enemies Target))))

(event `Update Still Alive`
  (params (Index :type Integer) (Exp :type "Float (double-precision)"))
  (`KismetSystemLibrary.Delay` 0.5)
  (`GameplayStatics.PlaySound2D` "/Game/GroupFolders/Mason/SFX/EnemyDeath.EnemyDeath" 1.0 1.0 0.0 null null)
  (`/Game/GroupFolders/Gabe/Battle_System/Blueprints/Battle_Ai/Mediator.Update Exp` (cast `/Game/GroupFolders/Gabe/Battle_System/Blueprints/Battle_Ai/Mediator` (`self.Mediator`) :!pure true) Exp)
  (`self.CheckParty`))

(event `CheckParty`
  (if (`self.Battle Over`)
    (set `/Game/GroupFolders/Gabe/Battle_System/RPG_GameInstance.First_Load` true (cast `/Game/GroupFolders/Gabe/Battle_System/RPG_GameInstance` (`GameplayStatics.GetGameInstance`) :!pure true))
    (set `self.Battle Over` false)
    (`/Game/GroupFolders/Gabe/Battle_System/Blueprints/Battle_Ai/Mediator.End_Battle` (cast `/Game/GroupFolders/Gabe/Battle_System/Blueprints/Battle_Ai/Mediator` (`self.Mediator`) :!pure true))
    (`KismetSystemLibrary.Delay` 0.2)
    (`GameplayStatics.OpenLevel` "WinScreen")))

(event `SuperMove`
  (params (`Player Stats` :type "/Game/GroupFolders/Gabe/Battle_System/Stats Structure") (`Player Weapon` :type "/Game/GroupFolders/Gabe/Battle_System/Weapon Structure"))
  (bind _enemies (`self.Enemies`))
  (set `self.Player Stats` `Player Stats`)
  (set `self.Player Weapon` `Player Weapon`)
  (`/Engine/EditorBlueprintResources/StandardMacros.IsValid` _enemies
    (:`Is Valid`
      (`self.Damage Calc` _enemies)
      (set `self.Damage` 0.0)
      (`KismetSystemLibrary.Delay` 1.0)
      (`self.Update Battle Msg`)
      (`KismetSystemLibrary.Delay` 5.0)
      (set `self.Damage` 0.0)
      (`Widget.RemoveFromParent` (`self.Battle Msg`))
      (`/Game/GroupFolders/Gabe/Battle_System/Blueprints/Battle_Ai/Mediator.Update PlayerTurn` (cast `/Game/GroupFolders/Gabe/Battle_System/Blueprints/Battle_Ai/Mediator` (`self.Mediator`) :!pure true)))))

(fn `Damage Calc`
  (params (Enemy :type "/Game/GroupFolders/Gabe/Battle_System/Blueprints/Battle_Ai/Ai_1-0/Boss Object Reference"))
  (bind _player_stats_attack (break `/Game/GroupFolders/Gabe/Battle_System/Stats` (`self.Player Stats`)))
  (bind (_player_weapon_name _player_weapon_damage _player_weapon_mod) (break `/Game/GroupFolders/Gabe/Battle_System/Weapon` (`self.Player Weapon`)))
  (bind (_player_weapon_name_2 _player_weapon_damage_2 _player_weapon_mod_2) (break `/Game/GroupFolders/Gabe/Battle_System/Weapon` (`self.Player Weapon`)))
  (bind (_stats_attack _stats_defense) (break `/Game/GroupFolders/Gabe/Battle_System/Stats` (`/Game/GroupFolders/Gabe/Battle_System/Blueprints/Battle_Ai/Ai_1-0/Boss.Stats` Enemy)))
  (bind _returnvalue (- _player_stats_attack _stats_defense))
  (if (> _returnvalue 0)
    (set `self.Damage` (`KismetMathLibrary.Conv_IntToDouble` (+ _player_weapon_mod_2 (* _player_weapon_damage _returnvalue))))
    (else
      (set `self.Damage` (`KismetMathLibrary.Conv_IntToDouble` (- (+ _player_weapon_damage _player_weapon_mod) (/ _stats_defense 2)))))))

(fn `Update Battle Msg`
  (bind _returnvalue (`|CreateWidget` "/Game/GroupFolders/Gabe/Battle_System/Widgets/BattleMsg.BattleMsg_C"))
  (bind _output_get (set `self.Battle Msg` _returnvalue))
  (set `/Game/GroupFolders/Gabe/Battle_System/Widgets/BattleMsg.Attacker` "Player" _output_get)
  (set `/Game/GroupFolders/Gabe/Battle_System/Widgets/BattleMsg.Reciver` "Enemy Party" _output_get)
  (set `/Game/GroupFolders/Gabe/Battle_System/Widgets/BattleMsg.Damage` (`self.Damage`) _output_get)
  (`/Game/GroupFolders/Gabe/Battle_System/Widgets/BattleMsg.Update` _output_get)
  (`UserWidget.AddToViewport` _output_get 0))

(fn `UserConstructionScript`)